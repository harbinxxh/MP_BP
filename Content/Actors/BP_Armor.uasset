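; BP_Armor is an armor pickup that equips itself on a player that overlaps it.
; On the server, overlap with any actor implementing BPI_Player triggers AttachMesh, then sends GrantedArmor through the interface's GrantArmorMessage.
; AttachMesh gets the player's mesh through the interface and snaps SphereMesh to its head socket and Cube to its spine socket.
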(event Collision|EventActorBeginOverlap
  (params (OtherActor :type Actor%20Object%20Reference))
  (Networking|SwitchHasAuthority
    (:Authority
      (if (Utilities|DoesObjectImplementInterface OtherActor "/Game/Interaction/BPI_Player.BPI_Player_C")
        (CallFunction|AttachMesh OtherActor)
        (Class|BPIPlayer|GrantArmor(Message) OtherActor (Variables|Default|GetGrantedArmor))))))

(fn ConstructionScript)

(fn AttachMesh
  (params (Object :type Object%20Object%20Reference))
  (bind _mesh (Class|BPIPlayer|GetMesh(Message) Object))
  (LocalVariables|SetAttachMesh _mesh)
  (Transformation|AttachComponentToComponent (Variables|Default|GetSphereMesh) (LocalVariables|GetAttachMesh) "S_Head" "SnapToTarget" "SnapToTarget" "SnapToTarget" true)
  (Transformation|AttachComponentToComponent (Variables|Default|GetCube) (LocalVariables|GetAttachMesh) "S_Spine" "SnapToTarget" "SnapToTarget" "SnapToTarget" true))
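; BP_GameState is a game state Blueprint that tracks membership of two teams.
; AddTeamMember keeps the teams balanced by adding each player to Team1 unless it has more members than Team2, so ties go to Team1.
; IsTeam1 reports whether a given player is in the Team1 array.
; The event graph and construction script contain no logic.
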(event EventBeginPlay)

(event EventTick
  (params (DeltaSeconds :type Float%20%28single-precision%29)))

(fn ConstructionScript)

(fn AddTeamMember
  (params (Player :type Player%20Controller%20Object%20Reference))
  (if (> (Utilities|Array|Length (Variables|Default|GetTeam%201)) (Utilities|Array|Length (Variables|Default|GetTeam%202)))
    (Utilities|Array|Add (Variables|Default|GetTeam%202) Player)
    (else
      (Utilities|Array|Add (Variables|Default|GetTeam%201) Player))))

(fn IsTeam1
  (params (Player :type Player%20Controller%20Object%20Reference))
  (return (Utilities|Array|ContainsItem (Variables|Default|GetTeam%201) Player)))